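; Crane part Blueprint that slides along the world X axis under player control, enabling input from player controller 0 on BeginPlay.
; Separate forward and backward axis inputs add or subtract a MovementSpeedX-scaled offset without sweep, each gated by its own pair of X bounds.
; Bounds are tested on the current position before moving, and the step is not scaled by delta time.
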(event EventBeginPlay
  (Input|EnableInput (Game|GetPlayerController 0)))

(event Input|AxisEvents|InputAxisMoveCraneForwards
  (params (AxisValue :type Float%20%28single-precision%29))
  (bind _returnvalue (Transformation|GetActorLocation))
  (bind _x (Math|Vector|BreakVector _returnvalue))
  (if (>= _x (Variables|Default|GetMovement_LowerBound_1))
    (if (<= _x (Variables|Default|GetMovement_UpperBound_1))
      (Transformation|SetActorLocation (+ (Transformation|GetActorLocation) (Math|Vector|MakeVector (* AxisValue (Variables|Default|GetMovement_Speed_X)) 0.0 0.0)) false false))))

(event Input|AxisEvents|InputAxisMoveCraneBackwards
  (params (AxisValue :type Float%20%28single-precision%29))
  (bind _returnvalue (Transformation|GetActorLocation))
  (bind _x (Math|Vector|BreakVector _returnvalue))
  (if (>= _x (Variables|Default|GetMovement_LowerBound_2))
    (if (<= _x (Variables|Default|GetMovement_UpperBound_2))
      (Transformation|SetActorLocation (- (Transformation|GetActorLocation) (Math|Vector|MakeVector (* AxisValue (Variables|Default|GetMovement_Speed_X)) 0.0 0.0)) false false))))

(fn ConstructionScript)