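; Crane part actor that the player moves vertically along Z to lower or raise it.
; It enables input from the first player controller on BeginPlay and handles the Lower Crane and Raise Crane axis events.
; Each event offsets the actor's location by axis value times a Z speed, without sweep or delta-time scaling, only while current Z lies within that direction's own pair of bounds.
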(event EventBeginPlay
  (Input|EnableInput (Game|GetPlayerController 0)))

(event Input|AxisEvents|InputAxisLowerCrane
  (params (AxisValue :type Float%20%28single-precision%29))
  (bind _returnvalue (Transformation|GetActorLocation))
  (bind _z (Math|Vector|BreakVector _returnvalue))
  (if (>= _z (Variables|Default|GetMovement_Lower_Bound_1))
    (if (<= _z (Variables|Default|GetMovement_Upper_Bound_1))
      (Transformation|SetActorLocation (- (Transformation|GetActorLocation) (Math|Vector|MakeVector 0.0 0.0 (* AxisValue (Variables|Default|GetMovement_Speed_Z)))) false false))))

(event Input|AxisEvents|InputAxisRaiseCrane
  (params (AxisValue :type Float%20%28single-precision%29))
  (bind _returnvalue (Transformation|GetActorLocation))
  (bind _z (Math|Vector|BreakVector _returnvalue))
  (if (>= _z (Variables|Default|GetMovement_Lower_Bound_2))
    (if (<= _z (Variables|Default|GetMovement_Upper_Bound_2))
      (Transformation|SetActorLocation (+ (Transformation|GetActorLocation) (Math|Vector|MakeVector 0.0 0.0 (* AxisValue (Variables|Default|GetMovement_Speed_Z)))) false false))))

(fn ConstructionScript)