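; Crane part actor that the player slides along the world Y axis with the Move Crane Left and Right input axes.
; It enables input from the first player controller on BeginPlay.
; Each axis event offsets the location by axis value times a speed variable, without sweep, only while the current Y lies within that direction's own lower and upper bounds.
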(event EventBeginPlay
  (Input|EnableInput (Game|GetPlayerController 0)))

(event Input|AxisEvents|InputAxisMoveCraneLeft
  (params (AxisValue :type Float%20%28single-precision%29))
  (bind _returnvalue (Transformation|GetActorLocation))
  (bind _y (Math|Vector|BreakVector _returnvalue))
  (if (>= _y (Variables|Default|GetMovement_Lower_Bound_1))
    (if (<= _y (Variables|Default|GetMovement_Upper_Bound_1))
      (Transformation|SetActorLocation (- (Transformation|GetActorLocation) (Math|Vector|MakeVector 0.0 (* AxisValue (Variables|Default|GetMovement_Speed_Y)) 0.0)) false false))))

(event Input|AxisEvents|InputAxisMoveCraneRight
  (params (AxisValue :type Float%20%28single-precision%29))
  (bind _returnvalue (Transformation|GetActorLocation))
  (bind _y (Math|Vector|BreakVector _returnvalue))
  (if (>= _y (Variables|Default|GetMovement_Lower_Bound_2))
    (if (<= _y (Variables|Default|GetMovement_Upper_Bound_2))
      (Transformation|SetActorLocation (+ (Transformation|GetActorLocation) (Math|Vector|MakeVector 0.0 (* AxisValue (Variables|Default|GetMovement_Speed_Y)) 0.0)) false false))))

(fn ConstructionScript)